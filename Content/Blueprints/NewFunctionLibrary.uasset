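; Blueprint function library of game helpers for item spawning and player scoring, sharing state through the first Database_Blueprint actor found.
; GetItemSpawnData picks random "item spawn" tagged actors, retries on matching the saved position, saves a position and returns a transform with ItemBeer.
; IncrementPlayerPoints raises one of four players' scores.
; SetMaxPlayerCount sets LocalMaxPlayer; its getter and GetThrowItemSpawnData are empty, with throw-spawn logic left unconnected.
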(fn GetItemSpawnData
  (Utilities|FlowControl|Sequence
    (:then_0
      ;[1 1 1] get spawn location
      (bind _outactors (Actor|GetAllActorswithTag 0 "item spawn" :!label _label))
      (bind _output (CallFunction|GetDatabase))
      (if (Math|Vector|Equal(Vector) (Variables|/Game/Blueprints/database_Blueprint.database_Blueprint_C|Getitem%20position _output) (Transformation|GetActorLocation (Utilities|Array|Get(acopy) _outactors (Math|Random|RandomIntegerinRange 0 (- (Utilities|Array|Length _outactors) 1)))) 0.0)
        (goto _label)
        (else
          (Variables|/Game/Blueprints/database_Blueprint.database_Blueprint_C|Setitem%20position _output (Transformation|GetActorLocation (Utilities|Array|Get(acopy) _outactors (Math|Random|RandomIntegerinRange 0 (- (Utilities|Array|Length _outactors) 1)))))
          (return (Math|Conversions|ToTransform(Vector) (Transformation|GetActorLocation (Utilities|Array|Get(acopy) _outactors (Math|Random|RandomIntegerinRange 0 (- (Utilities|Array|Length _outactors) 1))))) (LocalVariables|Getitem%20beer)))))))

(fn GetDatabase
  (bind _outactors (Actor|GetAllActorsOfClass 0 "/Game/Blueprints/database_Blueprint.database_Blueprint_C"))
  (return (Utilities|Array|Get(acopy) _outactors)))

(fn IncrementPlayerPoints
  (params (player%20num :type Integer))
  (bind _output (CallFunction|GetDatabase))
  (switch int (- player%20num 1)
    (:0
      (Math|Integer|IncrementInt (Variables|/Game/Blueprints/database_Blueprint.database_Blueprint_C|Getplayer1%20Points _output)))
    (:1
      (Math|Integer|IncrementInt (Variables|/Game/Blueprints/database_Blueprint.database_Blueprint_C|Getplayer2%20Points _output)))
    (:2
      (Math|Integer|IncrementInt (Variables|/Game/Blueprints/database_Blueprint.database_Blueprint_C|Getplayer3%20Points _output)))
    (:3
      (Math|Integer|IncrementInt (Variables|/Game/Blueprints/database_Blueprint.database_Blueprint_C|Getplayer4%20Points _output)))))

(fn SetMaxPlayerCount
  (params (Player%20count :type Integer))
  (LocalVariables|Setlocal%20max%20player Player%20count))

(fn GetLocalMaxPlayerCount)

(fn GetThrowItemSpawnData)