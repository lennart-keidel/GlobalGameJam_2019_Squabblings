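; Collectible pickup actor that slowly spins, scores a point event for whichever of four players touches it, then replaces itself.
; On overlap with a player-tagged actor, a cast chain over the four SquabblePlayableChar classes selects the player number passed to IncrementPlayerPoints.
; It then destroys itself and spawns a new Item_beer at the transform from GetItemSpawnData.
; Despite the beer name, the construction script gives each instance a random bubble-icon sprite, falling back to the remote icon.
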(event EventTick
  (params (DeltaSeconds :type Float%20%28single-precision%29))
  (Transformation|AddLocalRotation (Variables|Default|GetDefaultSceneRoot) "0,2.000000, 0" false false))

(event Collision|EventActorBeginOverlap
  (params (OtherActor :type Actor%20Object%20Reference))
  (if (Actor|ActorHasTag OtherActor "player")
    ;[1 1 1] destroy item, score
    (Utilities|Casting|CastToSquabblePlayableChar OtherActor
      (:then
        (CallFunction|IncrementPlayerPoints 1))
      (:CastFailed
        (Utilities|Casting|CastToSquabblePlayableChar1 OtherActor
          (:then
            (CallFunction|IncrementPlayerPoints 2))
          (:CastFailed
            (Utilities|Casting|CastToSquabblePlayableChar2 OtherActor
              (:then
                (CallFunction|IncrementPlayerPoints 3))
              (:CastFailed
                (Utilities|Casting|CastToSquabblePlayableChar3 OtherActor)
                (CallFunction|IncrementPlayerPoints 4)))))))
    (Actor|DestroyActor)
    ;[1 1 1] spawn next item
    (bind _returnvalue (CallFunction|GetItemSpawnData))
    (Game|SpawnActorfromClass "item_beer_C" _returnvalue "Undefined" 0 0)))

(fn ConstructionScript
  (bind _sprite (Variables|Default|GetSprite))
  (switch int (Math|Random|RandomIntegerinRange 0 (|GetNumEnumEntries))
    (:Default
      (Rendering|Components|Sprite|SetSprite _sprite "/Game/assets/Icons/RemoteBubbleIcon_Sprite.RemoteBubbleIcon_Sprite" :!label _label))
    (:0
      (Rendering|Components|Sprite|SetSprite _sprite "/Game/assets/Icons/BabyBottleBubbleIcon_Sprite.BabyBottleBubbleIcon_Sprite"))
    (:1
      (Rendering|Components|Sprite|SetSprite _sprite "/Game/assets/Icons/BeerBubbleIcon_Sprite.BeerBubbleIcon_Sprite"))
    (:2
      (Rendering|Components|Sprite|SetSprite _sprite "/Game/assets/Icons/BrickBubbleIcon_Sprite.BrickBubbleIcon_Sprite"))
    (:3
      (Rendering|Components|Sprite|SetSprite _sprite "/Game/assets/Icons/CakeBubbleIcon_Sprite.CakeBubbleIcon_Sprite"))
    (:4
      (Rendering|Components|Sprite|SetSprite _sprite "/Game/assets/Icons/CoffeeBubbleIcon_Sprite.CoffeeBubbleIcon_Sprite"))
    (:5
      (Rendering|Components|Sprite|SetSprite _sprite "/Game/assets/Icons/CookieBubbleIcon_Sprite.CookieBubbleIcon_Sprite"))
    (:6
      (Rendering|Components|Sprite|SetSprite _sprite "/Game/assets/Icons/DonutBubbleIcon_Sprite.DonutBubbleIcon_Sprite"))
    (:7
      (goto _label))))