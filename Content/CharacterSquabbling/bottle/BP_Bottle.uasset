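; Bottle pickup that the squabble playable characters grab by walking into its Sphere.
; On overlap it casts through four separate character classes and, if that character has no item, attaches to the mesh's "Lego" socket.
; It then disables Sphere collision and stores itself as the character's Item.
; Only the first two character branches set HasItem; the Char2 and Char3 branches leave it unchanged.
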(event OnComponentBeginOverlap(Sphere)
  (params (OverlappedComponent :type Primitive%20Component%20Object%20Reference) (OtherActor :type Actor%20Object%20Reference) (OtherComp :type Primitive%20Component%20Object%20Reference) (OtherBodyIndex :type Integer) (bFromSweep :type Boolean) (SweepResult :type Hit%20Result%20Structure%20%28by%20ref%29))
  (bind _assquabble_playable_char (Utilities|Casting|CastToSquabblePlayableChar OtherActor)
    (:then
      (if (not (Variables|/Game/CharacterSquabbling/SquabblePlayableChar.SquabblePlayableChar_C|GetHas%20Item? _assquabble_playable_char))
        (Variables|/Game/CharacterSquabbling/SquabblePlayableChar.SquabblePlayableChar_C|SetHas%20Item? _assquabble_playable_char true)
        (Transformation|AttachComponentToComponent (Variables|/Script/Engine.Character|GetMesh _assquabble_playable_char) "Lego" "SnapToTarget" "SnapToTarget" "SnapToTarget" false)
        (Collision|SetCollisionEnabled (Variables|Default|GetSphere) "NoCollision")
        (Variables|/Game/CharacterSquabbling/SquabblePlayableChar.SquabblePlayableChar_C|SetItem _assquabble_playable_char self)))
    (:CastFailed
      (bind _assquabble_playable_char_1 (Utilities|Casting|CastToSquabblePlayableChar1 OtherActor)
        (:then
          (if (not (Variables|/Game/CharacterSquabbling/SquabblePlayableChar1.SquabblePlayableChar1_C|GetHas%20Item? _assquabble_playable_char_1))
            (Variables|/Game/CharacterSquabbling/SquabblePlayableChar1.SquabblePlayableChar1_C|SetHas%20Item? _assquabble_playable_char_1 true)
            (Transformation|AttachComponentToComponent (Variables|/Script/Engine.Character|GetMesh _assquabble_playable_char_1) "Lego" "SnapToTarget" "SnapToTarget" "SnapToTarget" false)
            (Collision|SetCollisionEnabled (Variables|Default|GetSphere) "NoCollision")
            (Variables|/Game/CharacterSquabbling/SquabblePlayableChar1.SquabblePlayableChar1_C|SetItem _assquabble_playable_char_1 self)))
        (:CastFailed
          (bind _assquabble_playable_char_2 (Utilities|Casting|CastToSquabblePlayableChar2 OtherActor)
            (:then
              (if (not (Variables|/Game/CharacterSquabbling/SquabblePlayableChar2.SquabblePlayableChar2_C|GetHas%20Item? _assquabble_playable_char_2))
                (Transformation|AttachComponentToComponent (Variables|/Script/Engine.Character|GetMesh _assquabble_playable_char_2) "Lego" "SnapToTarget" "SnapToTarget" "SnapToTarget" false)
                (Collision|SetCollisionEnabled (Variables|Default|GetSphere) "NoCollision")
                (Variables|/Game/CharacterSquabbling/SquabblePlayableChar2.SquabblePlayableChar2_C|SetItem _assquabble_playable_char_2 self)))
            (:CastFailed
              (bind _assquabble_playable_char_3 (Utilities|Casting|CastToSquabblePlayableChar3 OtherActor))
              (if (not (Variables|/Game/CharacterSquabbling/SquabblePlayableChar3.SquabblePlayableChar3_C|GetHas%20Item? _assquabble_playable_char_3))
                (Transformation|AttachComponentToComponent (Variables|/Script/Engine.Character|GetMesh _assquabble_playable_char_3) "Lego" "SnapToTarget" "SnapToTarget" "SnapToTarget" false)
                (Collision|SetCollisionEnabled (Variables|Default|GetSphere) "NoCollision")
                (Variables|/Game/CharacterSquabbling/SquabblePlayableChar3.SquabblePlayableChar3_C|SetItem _assquabble_playable_char_3 self)))))))))

(event EventBeginPlay)

(event Collision|EventActorBeginOverlap
  (params (OtherActor :type Actor%20Object%20Reference)))

(event EventTick
  (params (DeltaSeconds :type Float%20%28single-precision%29)))

(fn ConstructionScript)